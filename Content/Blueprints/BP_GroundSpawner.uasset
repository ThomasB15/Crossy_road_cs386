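; BP_GroundSpawner builds the starting strip of BP_Ground tiles, grass followed by regular ground.
; On BeginPlay it places randomized grass tiles starting behind the player, then chains ground tiles, each at the previous tile's Spawnpoint component via NewestGround.
; Every tile receives a reference back to the spawner.
; A separate function spawns BP_Car at a given location with the same back-reference, but nothing here calls it.
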(event `self.ReceiveBeginPlay`
  (`self.SpawnInitialGround`))

(fn `Spawn Grass`
  (params (SpawnLoactaion :type "Vector Structure"))
  (bind _returnvalue (`|SpawnActorFromClass` "/Game/Blueprints/BP_Ground.BP_Ground_C" (`KismetMathLibrary.MakeTransform` SpawnLoactaion) "Undefined" "OverrideRootScale" null null))
  (bind _output_get (set `self.Newest Ground` _returnvalue))
  (set `/Game/Blueprints/BP_Ground.GroundSpawner` self _output_get)
  (`/Game/Blueprints/BP_Ground.GrassGround` _output_get)
  (`/Game/Blueprints/BP_Ground.RandomizeGround` _output_get))

(fn `Spawn Ground`
  (params (SpawnLoactaion :type "Vector Structure"))
  (bind _returnvalue (`|SpawnActorFromClass` "/Game/Blueprints/BP_Ground.BP_Ground_C" (`KismetMathLibrary.MakeTransform` SpawnLoactaion) "Undefined" "OverrideRootScale" null null))
  (bind _output_get (set `self.Newest Ground` _returnvalue))
  (set `/Game/Blueprints/BP_Ground.GroundSpawner` self _output_get))

(fn `spawncaratSpawnpoint`
  (params (SpawnLocation :type "Vector Structure"))
  (bind _returnvalue (`|SpawnActorFromClass` "/Game/Blueprints/BP_Car.BP_Car_C" (`KismetMathLibrary.MakeTransform` SpawnLocation) "Undefined" "OverrideRootScale" null null))
  (bind _output_get (set `self.Newest Car` _returnvalue))
  (set `/Game/Blueprints/BP_Car.CarSpawner` self _output_get)
  (`/Game/Blueprints/BP_Car.carGround` _output_get))

(fn `SpawnGrassAtSpawnpoint`
  (`self.Spawn Grass` (`SceneComponent.K2_GetComponentLocation` (`/Game/Blueprints/BP_Ground.spawnpoint` (`self.Newest Ground`)))))

(fn `SpawnGroundAtSpawnpoint`
  (`self.Spawn Ground` (`SceneComponent.K2_GetComponentLocation` (`/Game/Blueprints/BP_Ground.spawnpoint` (`self.Newest Ground`)))))

(fn `SpawnInitialGround`
  (for _ (range 4)
    (`/Engine/EditorBlueprintResources/StandardMacros.IsValid` (`self.Newest Ground`)
      (:`Is Valid`
        (`self.SpawnGrassAtSpawnpoint`))
      (:`Is Not Valid`
        (`self.Spawn Grass` (- (`self.K2_GetActorLocation` (`GameplayStatics.GetPlayerCharacter` 0)) (600.0 0.0 0.0))))))
  (for _ (range 18)
    (`/Engine/EditorBlueprintResources/StandardMacros.IsValid` (`self.Newest Ground`)
      (:`Is Valid`
        (`self.SpawnGroundAtSpawnpoint`))
      (:`Is Not Valid`
        (`self.Spawn Ground` (0.0 0.0 0.0))))))

(fn `UserConstructionScript`)