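; Ground spawner actor that lays down a chain of BP_Ground segments, starting at the player pawn's location.
; On BeginPlay it spawns a fixed initial run, placing each new segment at the SpawnPoint of the newest one.
; Each segment receives a reference back to the spawner, and the spawner tracks the latest as NewestGround to anchor the next spawn.
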(event `self.ReceiveBeginPlay`
  (`self.SpawnInitialGround`))

(fn `SpawnGround`
  (params (SpawnGround :type "Vector Structure"))
  (bind _returnvalue (`|SpawnActorFromClass` "/Game/blueprints/BP_Ground.BP_Ground_C" (`KismetMathLibrary.MakeTransform` SpawnGround) "Undefined" "OverrideRootScale" null null))
  (bind _output_get (set `self.NewestGround` _returnvalue))
  (set `/Game/blueprints/BP_Ground.GroundSpawner` self _output_get))

(fn `SpawnGroundAtSpawnPoint`
  (`self.SpawnGround` (`SceneComponent.K2_GetComponentLocation` (`/Game/blueprints/BP_Ground.SpawnPoint` (`self.NewestGround`)))))

(fn `SpawnInitialGround`
  (for _ (range 6)
    (`/Engine/EditorBlueprintResources/StandardMacros.IsValid` (`self.NewestGround`)
      (:`Is Valid`
        (`self.SpawnGroundAtSpawnPoint`))
      (:`Is Not Valid`
        (`self.SpawnGround` (`self.K2_GetActorLocation` (`GameplayStatics.GetPlayerPawn` 0)))))))

(fn `UserConstructionScript`)