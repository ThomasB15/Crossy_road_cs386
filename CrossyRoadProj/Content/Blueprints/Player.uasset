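; Player pawn for a Crossy Road-style chicken that hops a fixed step in four directions.
; Pressing a direction squashes the mesh; releasing restores it, sets target position and facing, and jumps.
; Tick interpolates toward both with a swept move, reverting the target when that fails and leaving Y uninterpolated while OnLog.
; The absolute-transform camera creeps along its local X by its X distance from the player, at fixed height.
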(event `self.ReceiveBeginPlay`
  (`SceneComponent.SetAbsolute` (`self.Camera`) true true false))

(event `self.ReceiveTick`
  (params (DeltaSeconds :type "Float (single-precision)"))
  (bind (_returnvalue_x _returnvalue_y _returnvalue_z) (`KismetMathLibrary.BreakVector` (`self.K2_GetActorLocation`)))
  (bind (_returnvalue_x_2 _returnvalue_y_2) (`KismetMathLibrary.BreakVector` (`KismetMathLibrary.VInterpTo_Constant` (`self.Location Placeholder`) (`self.NewPos`) DeltaSeconds 800.0)))
  (if (`self.OnLog`)
    (set `self.Location Placeholder` (`KismetMathLibrary.MakeVector` _returnvalue_x_2 _returnvalue_y _returnvalue_z))
    (else
      (bind _output_get (set `self.Location Placeholder` (`KismetMathLibrary.MakeVector` _returnvalue_x_2 _returnvalue_y_2 _returnvalue_z)))))
  (bind (_sweephitresult _returnvalue) (`self.K2_SetActorLocation` _output_get true))
  (if (not _returnvalue)
    (set `self.NewPos` (`self.LastPos`)))
  (`self.CameraMovement` DeltaSeconds)
  (bind _output_get_2 (set `self.Rotation Placeholder` (`KismetMathLibrary.RInterpTo_Constant` (`self.Rotation Placeholder`) (`self.New Rotation`) DeltaSeconds 500.0)))
  (`self.K2_SetActorRotation` _output_get_2))

(event `InputAction|Forward`
  (params (Key :type "Key Structure"))
  (bind _newpos (`self.NewPos`))
  (bind _chicken (`self.Chicken`))
  (bind _chicken_2 (`self.Chicken`))
  (bind (_returnvalue_x _returnvalue_y _returnvalue_z) (`KismetMathLibrary.BreakVector` (`SceneComponent.K2_GetComponentLocation` _chicken)))
  (bind (_returnvalue_x_2 _returnvalue_y_2 _returnvalue_z_2) (`KismetMathLibrary.BreakVector` (`SceneComponent.K2_GetComponentLocation` _chicken_2)))
  (:`Pressed`
    (`SceneComponent.SetWorldScale3D` _chicken (100.0 50.0 100.0) :!label _label)
    (`SceneComponent.K2_SetWorldLocation` _chicken (`KismetMathLibrary.MakeVector` _returnvalue_x _returnvalue_y (+ _returnvalue_z (`self.shiftUp`))) false false))
  (:`Released`
    (set `self.New Rotation` (struct))
    (set `self.LastPos` _newpos)
    (set `self.NewPos` (+ _newpos (`KismetMathLibrary.MakeVector` (`self.Move`))))
    (`self.Jump` :!label _label_2)
    (`SceneComponent.SetWorldScale3D` _chicken_2 (100.0 100.0 100.0))
    (`SceneComponent.K2_SetWorldLocation` _chicken_2 (`KismetMathLibrary.MakeVector` _returnvalue_x_2 _returnvalue_y_2 (- _returnvalue_z_2 (`self.shiftUp`))) false false)))

(event `InputAction|Back`
  (params (Key :type "Key Structure"))
  (bind _newpos (`self.NewPos`))
  (:`Pressed`
    (goto _label))
  (:`Released`
    (set `self.New Rotation` (struct :`Yaw` 180.0))
    (set `self.LastPos` _newpos)
    (set `self.NewPos` (+ _newpos (`KismetMathLibrary.MakeVector` (* (`self.Move`) -1.0))))
    (goto _label_2)))

(event `InputAction|Left`
  (params (Key :type "Key Structure"))
  (bind _newpos (`self.NewPos`))
  (:`Pressed`
    (goto _label))
  (:`Released`
    (set `self.New Rotation` (struct :`Yaw` 270.0))
    (set `self.LastPos` _newpos)
    (set `self.NewPos` (+ _newpos (`KismetMathLibrary.MakeVector` 0.0 (* (`self.Move`) -1.0))))
    (goto _label_2)))

(event `InputAction|Right`
  (params (Key :type "Key Structure"))
  (bind _newpos (`self.NewPos`))
  (:`Pressed`
    (goto _label))
  (:`Released`
    (set `self.New Rotation` (struct :`Yaw` 90.0))
    (set `self.LastPos` _newpos)
    (set `self.NewPos` (+ _newpos (`KismetMathLibrary.MakeVector` 0.0 (`self.Move`))))
    (goto _label_2)))

(fn `CameraMovement`
  (params (DeltaSeconds :type "Float (double-precision)"))
  (bind _returnvalue_x (`KismetMathLibrary.BreakVector` (`self.K2_GetActorLocation`)))
  (bind _camera (`self.Camera`))
  (bind (_returnvalue_x_2 _returnvalue_y) (`KismetMathLibrary.BreakVector` (`SceneComponent.K2_GetComponentLocation` _camera)))
  (bind _returnvalue_x_3 (`KismetMathLibrary.BreakVector` (`SceneComponent.K2_GetComponentLocation` (`self.Camera`))))
  (`SceneComponent.K2_AddLocalOffset` _camera (`KismetMathLibrary.MakeVector` (* (`KismetMathLibrary.Abs` (- _returnvalue_x_3 _returnvalue_x)) DeltaSeconds 0.01)) false false)
  (`SceneComponent.K2_SetWorldLocation` _camera (`KismetMathLibrary.MakeVector` _returnvalue_x_2 _returnvalue_y 550.0) false false))

(fn `UserConstructionScript`)