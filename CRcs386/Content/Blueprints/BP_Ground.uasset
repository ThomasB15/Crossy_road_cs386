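; BP_Ground is a ground tile actor for a spawner-driven level that extends as the player advances.
; When the Player overlaps its Triggerzone, it tells the GroundSpawner to spawn the next ground at a spawn point.
; RandomizeGround randomly sets the Grass mesh component to grass or road, while GrassGround always sets it to grass.
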(event `self.triggerzone.OnComponentBeginOverlap`
  (params (OverlappedComponent :type "PrimitiveComponent Object Reference") (OtherActor :type "Actor Object Reference") (OtherComp :type "PrimitiveComponent Object Reference") (OtherBodyIndex :type Integer) (bFromSweep :type Boolean) (SweepResult :type "HitResult Structure (by ref)"))
  (cast `/Game/Blueprints/Player` OtherActor)
  (`/Game/Blueprints/BP_GroundSpawner.SpawnGroundAtSpawnpoint` (`self.GroundSpawner`)))

(fn `GrassGround`
  (`StaticMeshComponent.SetStaticMesh` (`self.Grass`) (select `int` (`KismetMathLibrary.RandomIntegerInRange` 0) :`0` "/Game/Assets/Grass/grass.grass" :`1` "/Game/Assets/Grass/grass.grass" :!type "StaticMesh Object Reference")))

(fn `RandomizeGround`
  (`StaticMeshComponent.SetStaticMesh` (`self.Grass`) (select `int` (`KismetMathLibrary.RandomIntegerInRange` 0 1) :`0` "/Game/Assets/Grass/grass.grass" :`1` "/Game/Assets/road/road.road" :!type "StaticMesh Object Reference")))

(fn `UserConstructionScript`)