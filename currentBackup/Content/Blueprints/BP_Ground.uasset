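; Ground lane tile for a Crossy Road-style game that asks GroundSpawner for more ground when the player enters its trigger.
; RandomizeGround picks grass with decor, bare road, train track with an RL actor, or lowered river with lilypads or opposing log streams sharing a random speed multiplier.
; GrassGround forces a grass lane.
; Tick flags river lanes, where overlapping the water hitbox kills a player not on a log.
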(event `self.ReceiveTick`
  (params (DeltaSeconds :type "Float (single-precision)"))
  (if (> (`self.selection`) 8)
    (set `self.waterLane` true)))

(event `self.triggerzone.OnComponentBeginOverlap`
  (params (OverlappedComponent :type "PrimitiveComponent Object Reference") (OtherActor :type "Actor Object Reference") (OtherComp :type "PrimitiveComponent Object Reference") (OtherBodyIndex :type Integer) (bFromSweep :type Boolean) (SweepResult :type "HitResult Structure (by ref)"))
  (cast `/Game/Blueprints/Player` OtherActor)
  (`/Game/Blueprints/BP_GroundSpawner.SpawnGroundAtSpawnpoint` (`self.GroundSpawner`)))

(event `self.waterHB.OnComponentBeginOverlap`
  (params (OverlappedComponent :type "PrimitiveComponent Object Reference") (OtherActor :type "Actor Object Reference") (OtherComp :type "PrimitiveComponent Object Reference") (OtherBodyIndex :type Integer) (bFromSweep :type Boolean) (SweepResult :type "HitResult Structure (by ref)"))
  (bind _asplayer (cast `/Game/Blueprints/Player` OtherActor))
  (if (`self.waterLane`)
    (if (`/Game/Blueprints/Player.OnLog` _asplayer)
      _
      (elif (not (`/Game/Blueprints/Player.dead` _asplayer))
        (set `/Game/Blueprints/Player.dead` true _asplayer)
        (set `/Game/Blueprints/Player.water` true _asplayer)))))

(fn `GrassGround`
  (`StaticMeshComponent.SetStaticMesh` (`self.Grass`) (select `int` (`KismetMathLibrary.RandomIntegerInRange` 0) :`0` "/Game/Assets/Grass/grass.grass" :`1` "/Game/Assets/Grass/grass.grass" :!type "StaticMesh Object Reference"))
  (`self.SpawnGrassDecor`))

(fn `RandomizeGround`
  (bind _grass (`self.Grass`))
  (bind (_returnvalue_x _returnvalue_y _returnvalue_z) (`KismetMathLibrary.BreakVector` (`SceneComponent.K2_GetComponentLocation` _grass)))
  (bind _output_get (set `self.selection` (`KismetMathLibrary.RandomIntegerInRange` 0 10)))
  (`StaticMeshComponent.SetStaticMesh` (`self.Grass`) (select `int` _output_get :`0` "/Game/Assets/Grass/grass.grass" :`1` "/Game/Assets/Grass/grass.grass" :`2` "/Game/Assets/Grass/grass.grass" :`3` "/Game/Assets/Grass/grass.grass" :`4` "/Game/Assets/road/road.road" :`5` "/Game/Assets/road/road.road" :`6` "/Game/Assets/road/road.road" :`7` "/Game/Assets/road/road.road" :`8` "/Game/Assets/RR/traintrack2.traintrack2" :`9` "/Game/Assets/water/river.river" :`10` "/Game/Assets/water/river.river" :!type "StaticMesh Object Reference"))
  (if (< (`self.selection`) 4)
    (`self.SpawnGrassDecor`)
    (elif (== (`self.selection`) 8)
      (`self.SpawnRL`)
      (elif (> (`self.selection`) 8)
        (`SceneComponent.K2_SetWorldLocation` _grass (`KismetMathLibrary.MakeVector` _returnvalue_x _returnvalue_y (- _returnvalue_z 50.0)) false false)
        (if (== (`KismetMathLibrary.RandomIntegerInRange` 0 1) 0)
          (`self.SpawnLillypad`)
          (elif (== (`KismetMathLibrary.RandomIntegerInRange` 0 1) 0)
            (`self.SpawnLogs`)
            (else
              (`self.SpawnLogs2`))))))))

(fn `SpawnGrassDecor`
  (`|SpawnActorFromClass` "/Game/Blueprints/Decor.Decor_C" (`KismetMathLibrary.MakeTransform` (`SceneComponent.GetSocketLocation` (`self.sp1`) "None")) "Undefined" "OverrideRootScale" null null)
  (`|SpawnActorFromClass` "/Game/Blueprints/Decor.Decor_C" (`KismetMathLibrary.MakeTransform` (`SceneComponent.GetSocketLocation` (`self.sp2`) "None")) "Undefined" "OverrideRootScale" null null)
  (`|SpawnActorFromClass` "/Game/Blueprints/Decor.Decor_C" (`KismetMathLibrary.MakeTransform` (`SceneComponent.GetSocketLocation` (`self.sp6`) "None")) "Undefined" "OverrideRootScale" null null)
  (`|SpawnActorFromClass` "/Game/Blueprints/Decor.Decor_C" (`KismetMathLibrary.MakeTransform` (`SceneComponent.GetSocketLocation` (`self.sp7`) "None")) "Undefined" "OverrideRootScale" null null))

(fn `SpawnLillypad`
  (`|SpawnActorFromClass` "/Game/Blueprints/lillypad.lillypad_C" (`KismetMathLibrary.MakeTransform` (`SceneComponent.GetSocketLocation` (`self.sp1`) "None")) "Undefined" "OverrideRootScale" null null)
  (`|SpawnActorFromClass` "/Game/Blueprints/lillypad.lillypad_C" (`KismetMathLibrary.MakeTransform` (`SceneComponent.GetSocketLocation` (`self.sp2`) "None")) "Undefined" "OverrideRootScale" null null)
  (`|SpawnActorFromClass` "/Game/Blueprints/lillypad.lillypad_C" (`KismetMathLibrary.MakeTransform` (`SceneComponent.GetSocketLocation` (`self.sp6`) "None")) "Undefined" "OverrideRootScale" null null)
  (`|SpawnActorFromClass` "/Game/Blueprints/lillypad.lillypad_C" (`KismetMathLibrary.MakeTransform` (`SceneComponent.GetSocketLocation` (`self.sp7`) "None")) "Undefined" "OverrideRootScale" null null)
  (`|SpawnActorFromClass` "/Game/Blueprints/lillypad.lillypad_C" (`KismetMathLibrary.MakeTransform` (`SceneComponent.GetSocketLocation` (`self.sp5`) "None")) "Undefined" "OverrideRootScale" null null)
  (`|SpawnActorFromClass` "/Game/Blueprints/lillypad.lillypad_C" (`KismetMathLibrary.MakeTransform` (`SceneComponent.GetSocketLocation` (`self.sp3`) "None")) "Undefined" "OverrideRootScale" null null)
  (`|SpawnActorFromClass` "/Game/Blueprints/lillypad.lillypad_C" (`KismetMathLibrary.MakeTransform` (`SceneComponent.GetSocketLocation` (`self.sp4`) "None")) "Undefined" "OverrideRootScale" null null))

(fn `SpawnLogs`
  (bind (_returnvalue_x _returnvalue_y _returnvalue_z) (`KismetMathLibrary.BreakVector` (`SceneComponent.K2_GetComponentLocation` (`self.sp1`))))
  (bind _returnvalue (`|SpawnActorFromClass` "/Game/Blueprints/log.log_C" (`KismetMathLibrary.MakeTransform` (`KismetMathLibrary.MakeVector` _returnvalue_x _returnvalue_y _returnvalue_z)) "Undefined" "OverrideRootScale" null null))
  (bind _output_get (set `/Game/Blueprints/log.multiplier` (`KismetMathLibrary.RandomFloatInRange` 400.0 550.0) _returnvalue))
  (bind _returnvalue_2 (`|SpawnActorFromClass` "/Game/Blueprints/log.log_C" (`KismetMathLibrary.MakeTransform` (`KismetMathLibrary.MakeVector` _returnvalue_x (- _returnvalue_y (`KismetMathLibrary.RandomFloatInRange` 600.0 1200.0)) _returnvalue_z)) "Undefined" "OverrideRootScale" null null))
  (bind _output_get_2 (set `/Game/Blueprints/log.multiplier` _output_get _returnvalue_2))
  (bind _returnvalue_3 (`|SpawnActorFromClass` "/Game/Blueprints/log.log_C" (`KismetMathLibrary.MakeTransform` (`KismetMathLibrary.MakeVector` _returnvalue_x (- _returnvalue_y (`KismetMathLibrary.RandomFloatInRange` 1800.0 2400.0)) _returnvalue_z)) "Undefined" "OverrideRootScale" null null))
  (bind _output_get_3 (set `/Game/Blueprints/log.multiplier` _output_get_2 _returnvalue_3))
  (bind _returnvalue_4 (`|SpawnActorFromClass` "/Game/Blueprints/log.log_C" (`KismetMathLibrary.MakeTransform` (`KismetMathLibrary.MakeVector` _returnvalue_x (- _returnvalue_y (`KismetMathLibrary.RandomFloatInRange` 3000.0 3600.0)) _returnvalue_z)) "Undefined" "OverrideRootScale" null null))
  (bind _output_get_4 (set `/Game/Blueprints/log.multiplier` _output_get_3 _returnvalue_4))
  (bind _returnvalue_5 (`|SpawnActorFromClass` "/Game/Blueprints/log.log_C" (`KismetMathLibrary.MakeTransform` (`KismetMathLibrary.MakeVector` _returnvalue_x (- _returnvalue_y (`KismetMathLibrary.RandomFloatInRange` 4200.0 4800.0)) _returnvalue_z)) "Undefined" "OverrideRootScale" null null))
  (bind _output_get_5 (set `/Game/Blueprints/log.multiplier` _output_get_4 _returnvalue_5))
  (bind _returnvalue_6 (`|SpawnActorFromClass` "/Game/Blueprints/log.log_C" (`KismetMathLibrary.MakeTransform` (`KismetMathLibrary.MakeVector` _returnvalue_x (- _returnvalue_y (`KismetMathLibrary.RandomFloatInRange` 5400.0 6000.0)))) "Undefined" "OverrideRootScale" null null))
  (bind _output_get_6 (set `/Game/Blueprints/log.multiplier` _output_get_5 _returnvalue_6))
  (bind _returnvalue_7 (`|SpawnActorFromClass` "/Game/Blueprints/log.log_C" (`KismetMathLibrary.MakeTransform` (`KismetMathLibrary.MakeVector` _returnvalue_x (- _returnvalue_y (`KismetMathLibrary.RandomFloatInRange` 6600.0 7200.0)) _returnvalue_z)) "Undefined" "OverrideRootScale" null null))
  (bind _output_get_7 (set `/Game/Blueprints/log.multiplier` _output_get_6 _returnvalue_7))
  (bind _returnvalue_8 (`|SpawnActorFromClass` "/Game/Blueprints/log.log_C" (`KismetMathLibrary.MakeTransform` (`KismetMathLibrary.MakeVector` _returnvalue_x (- _returnvalue_y (`KismetMathLibrary.RandomFloatInRange` 7800.0 8400.0)) _returnvalue_z)) "Undefined" "OverrideRootScale" null null))
  (set `/Game/Blueprints/log.multiplier` _output_get_7 _returnvalue_8))

(fn `SpawnLogs2`
  (bind (_returnvalue_x _returnvalue_y _returnvalue_z) (`KismetMathLibrary.BreakVector` (`SceneComponent.K2_GetComponentLocation` (`self.sp7`))))
  (bind _returnvalue (`|SpawnActorFromClass` "/Game/Blueprints/log2.log2_C" (`KismetMathLibrary.MakeTransform` (`KismetMathLibrary.MakeVector` _returnvalue_x _returnvalue_y _returnvalue_z)) "Undefined" "OverrideRootScale" null null))
  (bind _output_get (set `/Game/Blueprints/log2.multiplier` (`KismetMathLibrary.RandomFloatInRange` 400.0 550.0) _returnvalue))
  (bind _returnvalue_2 (`|SpawnActorFromClass` "/Game/Blueprints/log2.log2_C" (`KismetMathLibrary.MakeTransform` (`KismetMathLibrary.MakeVector` _returnvalue_x (+ _returnvalue_y (`KismetMathLibrary.RandomFloatInRange` 600.0 1200.0)) _returnvalue_z)) "Undefined" "OverrideRootScale" null null))
  (bind _output_get_2 (set `/Game/Blueprints/log2.multiplier` _output_get _returnvalue_2))
  (bind _returnvalue_3 (`|SpawnActorFromClass` "/Game/Blueprints/log2.log2_C" (`KismetMathLibrary.MakeTransform` (`KismetMathLibrary.MakeVector` _returnvalue_x (+ _returnvalue_y (`KismetMathLibrary.RandomFloatInRange` 1800.0 2400.0)) _returnvalue_z)) "Undefined" "OverrideRootScale" null null))
  (bind _output_get_3 (set `/Game/Blueprints/log2.multiplier` _output_get_2 _returnvalue_3))
  (bind _returnvalue_4 (`|SpawnActorFromClass` "/Game/Blueprints/log2.log2_C" (`KismetMathLibrary.MakeTransform` (`KismetMathLibrary.MakeVector` _returnvalue_x (+ _returnvalue_y (`KismetMathLibrary.RandomFloatInRange` 3000.0 3600.0)) _returnvalue_z)) "Undefined" "OverrideRootScale" null null))
  (bind _output_get_4 (set `/Game/Blueprints/log2.multiplier` _output_get_3 _returnvalue_4))
  (bind _returnvalue_5 (`|SpawnActorFromClass` "/Game/Blueprints/log2.log2_C" (`KismetMathLibrary.MakeTransform` (`KismetMathLibrary.MakeVector` _returnvalue_x (+ _returnvalue_y (`KismetMathLibrary.RandomFloatInRange` 4200.0 4800.0)) _returnvalue_z)) "Undefined" "OverrideRootScale" null null))
  (bind _output_get_5 (set `/Game/Blueprints/log2.multiplier` _output_get_4 _returnvalue_5))
  (bind _returnvalue_6 (`|SpawnActorFromClass` "/Game/Blueprints/log2.log2_C" (`KismetMathLibrary.MakeTransform` (`KismetMathLibrary.MakeVector` _returnvalue_x (+ _returnvalue_y (`KismetMathLibrary.RandomFloatInRange` 5400.0 6000.0)) _returnvalue_z)) "Undefined" "OverrideRootScale" null null))
  (bind _output_get_6 (set `/Game/Blueprints/log2.multiplier` _output_get_5 _returnvalue_6))
  (bind _returnvalue_7 (`|SpawnActorFromClass` "/Game/Blueprints/log2.log2_C" (`KismetMathLibrary.MakeTransform` (`KismetMathLibrary.MakeVector` _returnvalue_x (+ _returnvalue_y (`KismetMathLibrary.RandomFloatInRange` 6600.0 7200.0)) _returnvalue_z)) "Undefined" "OverrideRootScale" null null))
  (bind _output_get_7 (set `/Game/Blueprints/log2.multiplier` _output_get_6 _returnvalue_7))
  (bind _returnvalue_8 (`|SpawnActorFromClass` "/Game/Blueprints/log2.log2_C" (`KismetMathLibrary.MakeTransform` (`KismetMathLibrary.MakeVector` _returnvalue_x (+ _returnvalue_y (`KismetMathLibrary.RandomFloatInRange` 7800.0 8400.0)) _returnvalue_z)) "Undefined" "OverrideRootScale" null null))
  (set `/Game/Blueprints/log2.multiplier` _output_get_7 _returnvalue_8))

(fn `SpawnRL`
  (`|SpawnActorFromClass` "/Game/Blueprints/RL.RL_C" (`KismetMathLibrary.MakeTransform` (`SceneComponent.GetSocketLocation` (`self.spRL`) "None")) "Undefined" "OverrideRootScale" null null))

(fn `UserConstructionScript`)